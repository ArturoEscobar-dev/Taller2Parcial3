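; Game mode for a two-player fighting game that ends the match when either fighter runs out of health.
; Each Tick casts both player characters to BP_Hero1, checking player 0's Player2Health first, then player 1's Player1Health.
; At zero or below, it shows the matching win widget, gives player 0's controller a cursor with UI-only input, and pauses the game.
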(event `self.ReceiveTick`
  (params (DeltaSeconds :type "Float (single-precision)"))
  (bind _returnvalue (`GameplayStatics.GetPlayerController` 0))
  (bind _returnvalue_2 (`GameplayStatics.GetPlayerController` 0))
  (bind _asbp_hero_1 (cast `/Game/ArturoEscobar/Sprites/Hero1/BluePrints/BP_Hero1` (`GameplayStatics.GetPlayerCharacter` 0)))
  (if (<= (`/Game/ArturoEscobar/Sprites/Hero1/BluePrints/BP_Hero1.Player2Health` _asbp_hero_1) 0.0)
    (bind _returnvalue_3 (`|CreateWidget` "/Game/Miguel/WB_PlayerWin1.WB_PlayerWin1_C"))
    (`UserWidget.AddToViewport` _returnvalue_3 0)
    (set `PlayerController.bShowMouseCursor` true _returnvalue_2)
    (`WidgetBlueprintLibrary.SetInputMode_UIOnlyEx` _returnvalue_2 null)
    (`GameplayStatics.SetGamePaused` true)
    (else
      (bind _asbp_hero_1_2 (cast `/Game/ArturoEscobar/Sprites/Hero1/BluePrints/BP_Hero1` (`GameplayStatics.GetPlayerCharacter` 1)))
      (if (<= (`/Game/ArturoEscobar/Sprites/Hero1/BluePrints/BP_Hero1.Player1Health` _asbp_hero_1_2) 0.0)
        (bind _returnvalue_4 (`|CreateWidget` "/Game/Miguel/WB_PlayerWin2.WB_PlayerWin2_C"))
        (`UserWidget.AddToViewport` _returnvalue_4 0)
        (set `PlayerController.bShowMouseCursor` true _returnvalue)
        (`WidgetBlueprintLibrary.SetInputMode_UIOnlyEx` _returnvalue null)
        (`GameplayStatics.SetGamePaused` true)))))

(fn `UserConstructionScript`)