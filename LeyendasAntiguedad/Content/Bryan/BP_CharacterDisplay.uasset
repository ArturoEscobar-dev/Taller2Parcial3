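; BP_CharacterDisplay is an actor that spawns one of two player characters, apparently as the back end of a character choice.
; P1Spawn, P2Spawn and RandomSpawn spawn BP_Character1 or Character2, then call Possess through player 0 character's LastHitBy controller, not GetPlayerController.
; RandomSpawn branches on a random integer, but its Max of 0 means it always picks BP_Character1.
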(event `P1Spawn`
  (bind _returnvalue (`|SpawnActorFromClass` "/Game/Bryan/BP_Character1.BP_Character1_C" (`KismetMathLibrary.MakeTransform` (0.0 0.0 0.0)) "Undefined" "OverrideRootScale" null null))
  (`Controller.Possess` (`Pawn.LastHitBy` (`GameplayStatics.GetPlayerCharacter` 0)) _returnvalue))

(event `P2Spawn`
  (bind _returnvalue (`|SpawnActorFromClass` "/Game/Bryan/Character2.Character2_C" (`KismetMathLibrary.MakeTransform` (0.0 0.0 0.0)) "Undefined" "OverrideRootScale" null null))
  (`Controller.Possess` (`Pawn.LastHitBy` (`GameplayStatics.GetPlayerCharacter` 0)) _returnvalue))

(event `RandomSpawn`
  (set `self.NewVar_0` (`KismetMathLibrary.RandomInteger` 0))
  (if (== (`self.NewVar_0`) 0)
    (bind _returnvalue (`|SpawnActorFromClass` "/Game/Bryan/BP_Character1.BP_Character1_C" (`KismetMathLibrary.MakeTransform` (0.0 0.0 0.0)) "Undefined" "OverrideRootScale" null null))
    (`Controller.Possess` (`Pawn.LastHitBy` (`GameplayStatics.GetPlayerCharacter` 0)) _returnvalue)
    (elif (== (`self.NewVar_0`) 1)
      (bind _returnvalue_2 (`|SpawnActorFromClass` "/Game/Bryan/Character2.Character2_C" (`KismetMathLibrary.MakeTransform` (0.0 0.0 0.0)) "Undefined" "OverrideRootScale" null null))
      (`Controller.Possess` (`Pawn.LastHitBy` (`GameplayStatics.GetPlayerCharacter` 0)) _returnvalue_2))))

(fn `UserConstructionScript`)